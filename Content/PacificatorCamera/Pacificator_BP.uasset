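; Pacificator camera actor that turns to watch the player character when it perceives one.
; Its AIPerception update stores a successfully sensed BP_ThirdPersonCharacter as Target and clears Target on any unsuccessful stimulus.
; While Target is valid, Tick smoothly interpolates the whole actor's rotation toward it using a look-at rotation.
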(event OnTargetPerceptionUpdated(AIPerception)
  (params (Actor :type Actor%20Object%20Reference) (Stimulus :type AI%20Stimulus%20Structure))
  (if (.bsuccessfullysensed Stimulus)
    (bind _asbp_third_person_character (Utilities|Casting|CastToBP_ThirdPersonCharacter Actor))
    (Variables|Default|SetTarget _asbp_third_person_character)
    (else
      (Variables|Default|SetTarget 0))))

(event EventBeginPlay)

(event EventTick
  (params (DeltaSeconds :type Float%20%28single-precision%29))
  (if (Utilities|IsValid (Variables|Default|GetTarget))
    (Transformation|SetActorRotation (Math|Interpolation|RInterpTo (Transformation|GetActorRotation) (Math|Rotator|FindLookatRotation (Transformation|GetActorLocation) (Transformation|GetActorLocation (Variables|Default|GetTarget))) DeltaSeconds 3.0))))

(fn ConstructionScript)
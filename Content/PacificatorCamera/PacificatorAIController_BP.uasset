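; AI controller for the Pacificator that detects the third-person player character and drives its behavior tree.
; It runs PacificatorBT on BeginPlay.
; On perception updates for the player character, it sets the Enemy and bEnemyInSight blackboard keys when sensed, and clears them when perception is lost.
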(event OnTargetPerceptionUpdated(AIPerception)
  (params (Actor :type Actor%20Object%20Reference) (Stimulus :type AI%20Stimulus%20Structure))
  (bind _asbp_third_person_character (Utilities|Casting|CastToBP_ThirdPersonCharacter Actor))
  (if (.bsuccessfullysensed Stimulus)
    (AI|Components|Blackboard|SetValueasObject (Variables|Default|GetBlackboard) (Utilities|Name|MakeLiteralName "Enemy") _asbp_third_person_character)
    (AI|Components|Blackboard|SetValueasBool (Variables|Default|GetBlackboard) (Utilities|Name|MakeLiteralName "bEnemyInSight") true)
    (else
      (AI|Components|Blackboard|SetValueasObject (Variables|Default|GetBlackboard) (Utilities|Name|MakeLiteralName "Enemy") 0)
      (AI|Components|Blackboard|SetValueasBool (Variables|Default|GetBlackboard) (Utilities|Name|MakeLiteralName "bEnemyInSight") false))))

(event EventBeginPlay
  (AI|RunBehaviorTree "/Game/PacificatorCamera/PacificatorBT.PacificatorBT"))

(fn ConstructionScript)
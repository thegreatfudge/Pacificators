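; MyProjectile_BP is a projectile Blueprint whose only active logic is a camera warp effect on its CameraBoom.
; The CameraWarp event picks a random starting rotation, then plays the CameraRandomValues timeline from the start.
; Each timeline update uses WarpValue to scale the boom's arm length and offset its relative rotation from that random base.
; BeginPlay, overlap, Tick and the construction script are empty.
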(event EventBeginPlay)

(event Collision|EventActorBeginOverlap
  (params (OtherActor :type Actor%20Object%20Reference)))

(event EventTick
  (params (DeltaSeconds :type Float%20%28single-precision%29)))

(event EventCameraWarp
  (bind _returnvalue (Math|Random|RandomFloatinRange -1.8e+02 1.8e+02))
  (Variables|Default|SetInitialRotation (Math|Rotator|MakeRotator _returnvalue _returnvalue _returnvalue))
  (bind _warpvalue (Timeline|Camera%20random%20values PlayFromStart)
    (:Update
      (Variables|/Script/Engine.SpringArmComponent|SetTargetArmLength (Variables|Default|GetCameraBoom) (* _warpvalue 2e+02))
      (Transformation|SetRelativeRotation (Variables|Default|GetCameraBoom) (Math|Rotator|MakeRotator (+ (.roll (Variables|Default|GetInitialRotation)) (* _warpvalue 2e+01)) (+ (.pitch (Variables|Default|GetInitialRotation)) (* _warpvalue 2e+01)) (+ (* _warpvalue 3e+01) (.yaw (Variables|Default|GetInitialRotation)))) false false))))

(fn ConstructionScript)